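; BP_Menu_3D is a world-placed menu actor with a widget, used to move the camera between linked menus.
; On BeginPlay it plays a music cue, binds to the Main_Menu_Widget transition event and disables its own collision.
; The widget's menu index selects an entry in LinkedMenus.
; A transition moves collision from this actor to the target and eases the player's view to it with SetViewTargetWithBlend.
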(event Custom|Transition_To
  (params (New:Menu :type BP%20Menu%203D%20Object%20Reference))
  (Collision|SetActorEnableCollision false)
  (Collision|SetActorEnableCollision New:Menu true)
  (Game|Player|SetViewTargetwithBlend (Game|GetPlayerController 0) New:Menu 4.0 "VTBlend_Linear" 2.0 false))

(event Custom|OnTransisionToMenues
  (params (MenuIndex :type Integer))
  (if (Utilities|Array|IsValidIndex (Variables|Default|GetLinkedMenus) MenuIndex)
    (CallFunction|Transitionto (Utilities|Array|Get(acopy) (Variables|Default|GetLinkedMenus) MenuIndex))))

(event EventBeginPlay
  (Audio|PlaySound2D "/Game/Menu/Slike/The_good_the_bad_and_the_ugly_Cue.The_good_the_bad_and_the_ugly_Cue" 1.0 1.0 1.0 0 0)
  (bind _asmain_menu_widget (Utilities|Casting|CastToMain_Menu_Widget (UserInterface|GetUserWidgetObject (Variables|Default|GetWidget))))
  (EventDispatchers|BindEventtoTransitionMenu _asmain_menu_widget (delegate Custom|OnTransisionToMenues))
  (Collision|SetActorEnableCollision false))

(fn ConstructionScript)