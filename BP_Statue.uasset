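; BP_Statue is an interactable statue actor that opens a web link when the player presses E nearby.
; The construction script adds a movable static mesh from the Mesh variable and applies InteractionBoxScale to the trigger box through a local transform.
; Overlapping the box shows a WBP_PressE prompt and enables input so E launches WebURL; ending overlap removes both.
; The overlap events do not check which actor triggered them.
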(event OnComponentBeginOverlap(Box)
  (params (OverlappedComponent :type Primitive%20Component%20Object%20Reference) (OtherActor :type Actor%20Object%20Reference) (OtherComp :type Primitive%20Component%20Object%20Reference) (OtherBodyIndex :type Integer) (bFromSweep :type Boolean) (SweepResult :type Hit%20Result%20Structure%20%28by%20ref%29))
  ;[1 1 1] On overlap show WBP_PressE then hide
  (bind _returnvalue (UserInterface|CreateWidget "/Game/NFT_Gallery_Pack_Vol1/Blueprints/WBP_PressE.WBP_PressE_C"))
  (UserInterface|Viewport|AddtoViewport _returnvalue 0)
  (Input|EnableInput (Game|GetPlayerController 0)))

(event OnComponentEndOverlap(Box)
  (params (OverlappedComponent :type Primitive%20Component%20Object%20Reference) (OtherActor :type Actor%20Object%20Reference) (OtherComp :type Primitive%20Component%20Object%20Reference) (OtherBodyIndex :type Integer))
  ;[1 1 1] On overlap show WBP_PressE then hide
  (Widget|RemovefromParent (stale OnComponentBeginOverlap(Box) _returnvalue))
  (Input|DisableInput (Game|GetPlayerController 0)))

(event EventBeginPlay)

(event Collision|EventActorBeginOverlap
  (params (OtherActor :type Actor%20Object%20Reference)))

(event EventTick
  (params (DeltaSeconds :type Float%20%28single-precision%29)))

(event Input|KeyboardEvents|E
  (params (Key :type Key%20Structure :default "None"))
  ;[1 1 1] Open URL
  (:Pressed
    (Utilities|Platform|LaunchURL (Variables|Default|Getweb%20URL))))

(fn ConstructionScript
  (bind _returnvalue (AddComponent|AddStaticMeshComponent false))
  (Transformation|SetMobility _returnvalue "Movable")
  (Components|StaticMesh|SetStaticMesh _returnvalue (Variables|Default|GetMesh))
  (Class|SceneComponent|AddLocalTransform (Variables|Default|GetBox) (Math|Transform|MakeTransform "0, 0, 0" "0, 0, 0" (Math|Conversions|ToVector(Float) (Variables|Default|GetInteraction%20box%20scale))) false false))